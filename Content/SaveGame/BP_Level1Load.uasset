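; BP_Level1Load is a trigger box that ends Level 1 when BP_NinjaBoy overlaps it.
; If the BP_SaveGame slot exists, it loads the save, sets Level1Complete, writes it back and opens Level2.
; If no save exists, it only saves a fresh BP_SaveGame object, without setting the flag or changing level.
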(event `self.Box.OnComponentBeginOverlap`
  (params (OverlappedComponent :type "PrimitiveComponent Object Reference") (OtherActor :type "Actor Object Reference") (OtherComp :type "PrimitiveComponent Object Reference") (OtherBodyIndex :type Integer) (bFromSweep :type Boolean) (SweepResult :type "HitResult Structure (by ref)"))
  (cast `/Game/Characters/BluePrints/MainCharacters/BP_NinjaBoy` OtherActor)
  (bind _returnvalue (`GameplayStatics.CreateSaveGameObject` "/Game/SaveGame/BP_SaveGame.BP_SaveGame_C"))
  (bind _output_get (set `self.SaveGame` _returnvalue))
  (bind _returnvalue_2 (`GameplayStatics.DoesSaveGameExist` "BP_SaveGame"))
  (if _returnvalue_2
    (bind _returnvalue_3 (`GameplayStatics.LoadGameFromSlot` "BP_SaveGame"))
    (bind _asbp_save_game (cast `/Game/SaveGame/BP_SaveGame` _returnvalue_3))
    (bind _output_get_2 (set `self.SaveGameInstance` _asbp_save_game))
    (set `/Game/SaveGame/BP_SaveGame.Level1Complete` true _output_get_2)
    (`GameplayStatics.SaveGameToSlot` _output_get_2 "BP_SaveGame")
    (`GameplayStatics.OpenLevel` "Level2")
    (else
      (`GameplayStatics.SaveGameToSlot` _output_get "BP_SaveGame"))))

(fn `UserConstructionScript`)