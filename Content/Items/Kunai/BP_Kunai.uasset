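; BP_Kunai is a kunai actor that BP_NinjaBoy can pick up to refill its kunai count.
; It destroys itself five seconds after BeginPlay unless collected earlier.
; A capsule overlap while JustShot is set only clears that flag after a short delay, guarding against instant pickup after firing.
; Otherwise, overlapping a BP_NinjaBoy below MaxKunaiCapacity adds one kunai and destroys the actor.
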(event `self.ReceiveBeginPlay`
  (`KismetSystemLibrary.Delay` 5.0)
  (`self.K2_DestroyActor`))

(event `self.Capsule.OnComponentBeginOverlap`
  (params (OverlappedComponent :type "PrimitiveComponent Object Reference") (OtherActor :type "Actor Object Reference") (OtherComp :type "PrimitiveComponent Object Reference") (OtherBodyIndex :type Integer) (bFromSweep :type Boolean) (SweepResult :type "HitResult Structure (by ref)"))
  (if (`self.JustShot`)
    (`KismetSystemLibrary.Delay` 0.2)
    (set `self.JustShot` false)
    (else
      (bind _asbp_ninja_boy (cast `/Game/Characters/BluePrints/MainCharacters/BP_NinjaBoy` OtherActor))
      (bind _kunai (`/Game/Characters/BluePrints/MainCharacters/BP_NinjaBoy.Kunai` _asbp_ninja_boy))
      (if (< _kunai (`/Game/Characters/BluePrints/MainCharacters/BP_NinjaBoy.MaxKunaiCapacity` _asbp_ninja_boy))
        (set `/Game/Characters/BluePrints/MainCharacters/BP_NinjaBoy.Kunai` (+ _kunai 1.0) _asbp_ninja_boy)
        (`self.K2_DestroyActor`)))))

(fn `UserConstructionScript`)